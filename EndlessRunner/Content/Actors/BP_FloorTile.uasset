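; BP_FloorTile is a floor tile actor that randomly populates itself with pickups and obstacles and exposes an attach point transform, apparently for chaining tiles.
; The construction script rolls weighted chances to add five random pickups and one random obstacle as child actors within their spawn-zone boxes.
; Any overlap with its trigger box fires the Exited dispatcher; the delayed self-destroy logic is disconnected.
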(event `self.Box.OnComponentBeginOverlap`
  (params (OverlappedComponent :type "PrimitiveComponent Object Reference") (OtherActor :type "Actor Object Reference") (OtherComp :type "PrimitiveComponent Object Reference") (OtherBodyIndex :type Integer) (bFromSweep :type Boolean) (SweepResult :type "HitResult Structure (by ref)"))
  (`self.Exited` self))

(fn `GenerateRandomObjectPoints`
  (params (PickupNumber :type Integer :default 3))
  (returns (SpawnPointObject :type "Array of Vector Structure"))
  (bind _spawnzoneobjects (`self.SpawnZoneObjects`))
  (bind _output_get (set `self.Pickup Number` PickupNumber))
  (bind _result (`/Engine/EditorBlueprintResources/StandardMacros.DecrementInt` _output_get)
    (:`  `
      (for _index (range (+ _result 1))
        (`KismetArrayLibrary.Array_Insert` (`self.Spawn Point Object`) (`KismetMathLibrary.RandomPointInBoundingBox` (`SceneComponent.RelativeLocation` _spawnzoneobjects) (`BoxComponent.BoxExtent` _spawnzoneobjects)) _index))
      (return (`self.Spawn Point Object`)))))

(fn `GenerateRandomObstaclePoint`
  (returns (SpawnPointObstacle :type "Vector Structure"))
  (bind _spawnzoneobstacle (`self.SpawnZoneObstacle`))
  (return (`KismetMathLibrary.RandomPointInBoundingBox` (`SceneComponent.RelativeLocation` _spawnzoneobstacle) (`BoxComponent.BoxExtent` _spawnzoneobstacle))))

(fn `GetAttachTransform`
  (returns (AttachTransform :type "Transform Structure"))
  (return (`SceneComponent.K2_GetComponentToWorld` (`self.AttachPoint`))))

(fn `Spawn Obstacle`
  (bind _spawnpointobstacle (`self.GenerateRandomObstaclePoint` self))
  (bind _returnvalue (`AddComponent|NODE_AddChildActorComponent-1` :`RelativeTransform` (`KismetMathLibrary.Conv_VectorToTransform` _spawnpointobstacle)))
  (`ChildActorComponent.SetChildActorClass` _returnvalue (`KismetArrayLibrary.Array_Random` (`self.ObstacleType`))))

(fn `SpawnObjects`
  (bind _spawnpointobject (`self.GenerateRandomObjectPoints` self 5))
  (for _array_element _spawnpointobject
    (bind _returnvalue (`AddComponent|NODE_AddChildActorComponent-2` :`self` self :`RelativeTransform` (`KismetMathLibrary.Conv_VectorToTransform` _array_element)))
    (`ChildActorComponent.SetChildActorClass` _returnvalue (`KismetArrayLibrary.Array_Random` (`self.ObjectType`)))))

(fn `UserConstructionScript`
  (`|ExecutionSequence`
    (:`then_0`
      (if (`KismetMathLibrary.RandomBoolWithWeight` (`self.PickupSpawnChance`))
        (`self.SpawnObjects` self)))
    (:`then_1`
      (if (`KismetMathLibrary.RandomBoolWithWeight` (`self.ObstacleSpawnChance`))
        (`self.Spawn Obstacle` self)))))