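; Player character Blueprint for what appears to be a runner game, handling death and coin pickup through two custom events.
; Die runs once: it stops movement, disables input, plays an explosion sound and effect at the pawn, hides the mesh, then restarts the level by console command after a delay.
; CollectCoin increments the coin counter, prints it on screen and plays an optional 2D sound.
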(event `Die`
  (bind _returnvalue (`self.K2_GetActorLocation` (`GameplayStatics.GetPlayerPawn` 0)))
  (`/Engine/EditorBlueprintResources/StandardMacros.DoOnce` false
    (:`Completed`
      (`|ExecutionSequence`
        (:`then_0`
          ;[1 1 1] Stop Mooving
          (set `CharacterMovementComponent.MaxWalkSpeed` 0.0 (`self.CharacterMovement`)))
        (:`then_1`
          ;[1 1 1] Disable Inputs
          (`self.DisableInput` (`GameplayStatics.GetPlayerController` 0)))
        (:`then_2`
          ;[1 1 1] VFX Explosion
          (`GameplayStatics.PlaySoundAtLocation` "/Game/StarterContent/Audio/Explosion01.Explosion01" _returnvalue (struct) 1.0 1.0 0.0 null null null null)
          (`GameplayStatics.SpawnEmitterAtLocation` "/Game/StarterContent/Particles/P_Explosion.P_Explosion" _returnvalue))
        (:`then_3`
          ;[1 1 1] Hide Character
          (`SceneComponent.SetVisibility` (`self.Mesh`) false false))
        (:`then_4`
          ;[1 1 1] Restart Level
          (`KismetSystemLibrary.Delay` 3.0)
          (`KismetSystemLibrary.ExecuteConsoleCommand` "RestartLevel" null))))))

(event `CollectCoin`
  (bind _result (`/Engine/EditorBlueprintResources/StandardMacros.IncrementInt` (`self.CoinCollected`))
    (:`  `
      (bind _output_get (set `self.CoinCollected` _result))
      (`KismetSystemLibrary.PrintString` (`KismetStringLibrary.Conv_IntToString` _output_get) true false (struct :`R` 1.0 :`G` 0.95192 :`A` 1.0) 1.0)
      (bind _sound (`self.Sound`)
        (:`then`
          (`GameplayStatics.PlaySound2D` _sound 1.0 1.0 0.0 null null))
        (:`else`)))))

(fn `UserConstructionScript`)