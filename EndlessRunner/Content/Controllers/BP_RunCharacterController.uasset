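; BP_RunCharacterController is a controller Blueprint that drives a possessed BP_RunCharacter with basic movement input.
; On BeginPlay it casts the controlled pawn to BP_RunCharacter and caches the reference.
; The MoveForward and MoveRight axis events feed AddMovementInput along that character's forward and right vectors, scaled by the axis value.
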(event `self.ReceiveBeginPlay`
  (bind _asbp_run_character (cast `/Game/Actors/BP_RunCharacter` (`self.K2_GetPawn`)))
  (set `self.RunCharacter` _asbp_run_character))

(event `InputAxis|MoveForward`
  (params (AxisValue :type "Float (single-precision)"))
  (bind _runcharacter (`self.RunCharacter`))
  (`Pawn.AddMovementInput` _runcharacter (`self.GetActorForwardVector` _runcharacter) AxisValue false))

(event `InputAxis|MoveRight`
  (params (AxisValue :type "Float (single-precision)"))
  (bind _runcharacter (`self.RunCharacter`))
  (`Pawn.AddMovementInput` _runcharacter (`self.GetActorRightVector` _runcharacter) AxisValue false))

(fn `UserConstructionScript`)