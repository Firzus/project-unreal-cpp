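; BP_RunGameMode is the game mode for an endless runner, spawning floor tiles and driving the player pawn forward.
; BeginPlay spawns an initial run of tiles sized by TileNumber, chaining each BP_FloorTile onto the previous one's attach transform.
; Each tile's Exited event spawns a replacement at the end, then destroys the exited tile after a short delay.
; Tick feeds constant forward movement input to the player pawn.
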(event `self.ReceiveBeginPlay`
  (bind _result (`/Engine/EditorBlueprintResources/StandardMacros.DecrementInt` (`self.TileNumber`))
    (:`  `
      (for _ (range (+ _result 1))
        (`self.SpawnNextTile`)))))

(event `TileExited`
  (params (Tile :type "/Game/Actors/BP_FloorTile Object Reference"))
  (`self.SpawnNextTile`)
  (`KismetSystemLibrary.Delay` 1.0)
  (`self.K2_DestroyActor` Tile))

(event `self.ReceiveTick`
  (params (DeltaSeconds :type "Float (single-precision)"))
  (bind _returnvalue (`GameplayStatics.GetPlayerPawn` 0))
  ;[1 1 1] Infinite Forward Run
  (`Pawn.AddMovementInput` _returnvalue (`self.GetActorForwardVector` _returnvalue) 1.0 false))

(fn `SpawnNextTile`
  (bind _returnvalue (`|SpawnActorFromClass` "/Game/Actors/BP_FloorTile.BP_FloorTile_C" (`self.NextTileTransform`) "Undefined" "MultiplyWithRoot" null null))
  (add `/Game/Actors/BP_FloorTile.Exited` _returnvalue (`|CreateDelegate` :!event `TileExited`))
  (bind _attachtransform (`/Game/Actors/BP_FloorTile.GetAttachTransform` _returnvalue))
  (set `self.NextTileTransform` _attachtransform))

(fn `UserConstructionScript`)